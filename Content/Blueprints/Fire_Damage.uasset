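; Fire hazard actor that damages the player over time and ends the game once its trigger box is entered.
; BeginPlay caches the player as MyChar, and a box overlap by that player starts a delayed loop that repeatedly subtracts Health.
; The loop does not check Health or overlap exit; on completion it always shows the GameOverUI widget and pauses the game.
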(event `self.ReceiveBeginPlay`
  (bind _asmy_char (cast `/Game/Character/MyChar` (`GameplayStatics.GetPlayerCharacter` 0)))
  (set `self.As My Char` _asmy_char))

(event `self.Box.OnComponentBeginOverlap`
  (params (OverlappedComponent :type "PrimitiveComponent Object Reference") (OtherActor :type "Actor Object Reference") (OtherComp :type "PrimitiveComponent Object Reference") (OtherBodyIndex :type Integer) (bFromSweep :type Boolean) (SweepResult :type "HitResult Structure (by ref)"))
  (bind _as_my_char (`self.As My Char`))
  (if (== OtherActor (`GameplayStatics.GetPlayerCharacter` 0))
    (`/Game/Blueprints/Custom_Loop.For_Loop_With_Delay` 0 8 1.0
      (:`Body`
        (set `/Game/Character/MyChar.Health` (- (`/Game/Character/MyChar.Health` _as_my_char) 10) _as_my_char))
      (:`Completed`
        (bind _returnvalue (`|CreateWidget` "/Game/UI/GameOverUI.GameOverUI_C"))
        (`UserWidget.AddToViewport` _returnvalue 0)
        (`GameplayStatics.SetGamePaused` true)))))

(fn `UserConstructionScript`)